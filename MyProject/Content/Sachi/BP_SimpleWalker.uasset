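; BP_SimpleWalker is a player-controlled pawn that wanders the navmesh on its own.
; On BeginPlay it caches its PlayerController and starts a looping timer that fires Jumpp every few seconds.
; Despite its name, Jumpp uses SimpleMoveToLocation toward a random navigable point around player 0's pawn.
; A Box overlap prints a collision message to screen only when the other actor's class is BP_mySpawnedActor.
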(event `self.ReceiveBeginPlay`
  (bind _asplayer_controller (cast `PlayerController` (`self.GetController`)))
  (`KismetSystemLibrary.K2_SetTimerDelegate` (delegate `Jumpp`) 3.0 true))

(event `Jumpp`
  (bind _randomlocation (`NavigationSystemV1.K2_GetRandomLocationInNavigableRadius` (`self.K2_GetActorLocation` (`GameplayStatics.GetPlayerPawn` 0)) 2000.0 null null))
  (`AIBlueprintHelperLibrary.SimpleMoveToLocation` (stale `self.ReceiveBeginPlay` _asplayer_controller) _randomlocation))

(event `self.Box.OnComponentBeginOverlap`
  (params (OverlappedComponent :type "PrimitiveComponent Object Reference") (OtherActor :type "Actor Object Reference") (OtherComp :type "PrimitiveComponent Object Reference") (OtherBodyIndex :type Integer) (bFromSweep :type Boolean) (SweepResult :type "HitResult Structure (by ref)"))
  (`KismetSystemLibrary.PrintText` "Collided" (== (`GameplayStatics.GetObjectClass` OtherActor) "/Game/Sachi/BP_mySpawnedActor.BP_mySpawnedActor_C")))

(fn `UserConstructionScript`)